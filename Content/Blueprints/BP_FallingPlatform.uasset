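; Falling platform that drops after the player character steps on it, then returns to its starting place and re-arms.
; An overlap on the Box trigger starts a delayed sequence guarded by an Active flag, enabling physics on the Cube, then disabling it.
; A timeline lerps the Cube back to the transform saved at BeginPlay, playing a sound every update and on finish.
; Material swaps color each phase: warning, falling, resetting and ready.
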(event OnComponentBeginOverlap(Box)
  (params (OverlappedComponent :type Primitive%20Component%20Object%20Reference) (OtherActor :type Actor%20Object%20Reference) (OtherComp :type Primitive%20Component%20Object%20Reference) (OtherBodyIndex :type Integer) (bFromSweep :type Boolean) (SweepResult :type Hit%20Result%20Structure%20%28by%20ref%29))
  (bind _cube (Variables|Default|GetCube))
  (bind _starting_transform (Variables|Default|GetStarting%20Transform))
  (Utilities|Casting|CastToBP_ThirdPersonCharacter OtherActor) ; Is it the player that is standing on us?
  (if (not (Variables|Default|GetActive)) ; are we doing things?
    (Variables|Default|SetActive true) ; No? Well let's do things now!
    (Rendering|Material|SetMaterial (Variables|Default|GetCube) 0 "/AnimationSharing/AnimSharingBlue.AnimSharingBlue") ; Turning Blue because we're about to fall
    (Utilities|FlowControl|Delay 1.0)
    (Rendering|Material|SetMaterial (Variables|Default|GetCube) 0 "/AnimationSharing/AnimSharingRed.AnimSharingRed") ; Turning red beacuse we're falling now.
    (Physics|SetSimulatePhysics (Variables|Default|GetCube) true)
    (Utilities|FlowControl|Delay 4.0)
    (Rendering|Material|SetMaterial (Variables|Default|GetCube) 0 "/AnimationSharing/AnimSharingGreen.AnimSharingGreen") ; Turning green because we are resetting
    (Physics|SetSimulatePhysics _cube false)
    (bind _output_get (Variables|Default|SetLastRestingTransform (Transformation|GetWorldTransform _cube)))
    (bind _newtrack_0 (Timeline|LerpBackToStart PlayFromStart)
      (:Update
        (Transformation|SetWorldTransform (Variables|Default|GetCube) (Math|Transform|MakeTransform (Math|Vector|Lerp(Vector) (.location _output_get) (.location _starting_transform) _newtrack_0) (Math|Rotator|Lerp(Rotator) (.rotation _output_get) (.rotation _starting_transform) _newtrack_0) (.scale _starting_transform)) false false)
        (Audio|PlaySoundatLocation "/Game/QuestionMark/bleepbloops.bleepbloops" "0, 0, 0" "0, 0, 0" 1.0 1.0 0.0 "/Game/QuestionMark/NewSoundAttenuation.NewSoundAttenuation" 0 0 0))
      (:Finished
        (Rendering|Material|SetMaterial (Variables|Default|GetCube) 0 (Variables|Default|GetStartingMaterial)) ; Turning white because we're ready to go again.
        (Variables|Default|SetActive false)
        (Audio|PlaySoundatLocation "/Game/QuestionMark/bleepbloops.bleepbloops" "0, 0, 0" "0, 0, 0" 1.0 1.0 0.0 "/Game/QuestionMark/NewSoundAttenuation.NewSoundAttenuation" 0 0 0)))))

(event EventBeginPlay
  (Variables|Default|SetStarting%20Transform (Transformation|GetWorldTransform (Variables|Default|GetCube)))
  (Variables|Default|SetStartingMaterial (Rendering|Material|GetMaterial (Variables|Default|GetCube) 0)))

(fn ConstructionScript)